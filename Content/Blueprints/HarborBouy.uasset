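; Harbor buoy actor that rings a bell as it tips and drives level progression or game over through the volumes it touches.
; Tick checks the mesh's up vector and, when tilted past a small threshold, plays a random bell sound, throttled by a DoOnce reset after a delay.
; Overlapping IncreaseLevel_Blueprint calls LaunchBouy on the game mode and destroys the buoy.
; Overlapping GameOver_Blueprint flags game over on the HUD, then loads the main menu after a pause.
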(event EventTick
  (params (DeltaSeconds :type Float%20%28single-precision%29))
  (bind _staticmeshcomponent (Variables|Default|GetStaticMeshComponent))
  (bind _bellsounds (Variables|Default|GetBellSounds))
  (bind _returnvalue (Transformation|GetWorldRotation _staticmeshcomponent))
  (bind _returnvalue_2 (Math|Vector|GetUpVector _returnvalue))
  (bind (_x _y) (Math|Vector|BreakVector _returnvalue_2))
  (if (not (and (Math|Float|InRange(Float) _x -0.2 0.2) (Math|Float|InRange(Float) _y -0.2 0.2)))
    (Utilities|FlowControl|DoOnce false :!label _label
      (:Completed
        (Audio|PlaySoundatLocation (Utilities|Array|Get(acopy) _bellsounds (Math|Random|RandomIntegerinRange 0 (Utilities|Array|Length _bellsounds))) (Transformation|GetWorldLocation (Variables|Default|GetStaticMeshComponent)) "0, 0, 0" 0.8)
        (Utilities|FlowControl|Delay 0.9)
        (goto _label Reset)))))

(event Collision|EventActorBeginOverlap
  (params (OtherActor :type Actor%20Object%20Reference))
  (Utilities|Casting|CastToIncreaseLevel_Blueprint OtherActor
    (:then
      (bind _asmy_game_mode (Utilities|Casting|CastTomyGameMode (Game|GetGameMode)))
      (Default|LaunchBouy _asmy_game_mode)
      (Actor|DestroyActor))
    (:CastFailed
      (Utilities|Casting|CastToGameOver_Blueprint OtherActor)
      (bind _asmy_hud (Utilities|Casting|CastTomyHUD (HUD|GetHUD (Game|GetPlayerController 0))))
      (Variables|/Game/Blueprints/myHUD.myHUD_C|SetgameOver _asmy_hud true)
      (Utilities|FlowControl|Delay 4.0)
      (Game|OpenLevel(byName) "MainMenuMap"))))

(fn ConstructionScript
  (|CallParentFunction))