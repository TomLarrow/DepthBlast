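; myHUD is a HUD Blueprint that draws the player's wave and explosion counts and a game-over message.
; On BeginPlay it caches the game mode, cast to myGameMode.
; Each DrawHUD call draws text from that mode's Level and BarrelsUsed values at the top-left, plus a large "Game Over" label when the GameOver flag is set.
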(event EventDrawHUD
  (params (SizeX :type Integer) (SizeY :type Integer))
  (bind _mygamemode (Variables|Default|GetmyGameMode))
  (HUD|DrawText (Utilities|String|Append "Wave: " (Utilities|String|ToString(Integer) (Variables|/Game/Blueprints/myGameMode.myGameMode_C|Getlevel _mygamemode))) "(R=0,G=0,B=0,A=1)" 5.0 5.0 "/Game/myFont.myFont" 1.0 false)
  (HUD|DrawText (Utilities|String|Append "Explosions: " (Utilities|String|ToString(Integer) (Variables|/Game/Blueprints/myGameMode.myGameMode_C|GetBarrelsUsed _mygamemode))) "(R=0,G=0,B=0,A=1)" 5.0 25.0 "/Game/myFont.myFont" 1.0 false)
  (if (Variables|Default|GetgameOver)
    (HUD|DrawText "Game Over" "(R=0,G=0,B=0,A=1)" 1.8e+02 1.8e+02 "/Game/largeFont.largeFont" 1.0 true)))

(event EventBeginPlay
  (bind _asmy_game_mode (Utilities|Casting|CastTomyGameMode (Game|GetGameMode)))
  (Variables|Default|SetmyGameMode _asmy_game_mode))

(fn ConstructionScript)